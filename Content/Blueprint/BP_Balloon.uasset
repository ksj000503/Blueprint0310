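; BP_Balloon is a balloon actor that rises along its up vector and destroys itself above a fixed world height.
; Each Tick rerolls a random move speed, scales it by delta time and moves the actor without sweeping, so the climb rate varies per frame.
; An OnRep handler for BalloonVector exists but is empty, as is the construction script.
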(event `self.ReceiveTick`
  (params (DeltaSeconds :type "Float (single-precision)"))
  (bind _output_get (set `self.MoveSpeed` (`KismetMathLibrary.RandomFloatInRange` 50.0 500.0)))
  (`self.K2_SetActorLocation` (+ (* (* DeltaSeconds _output_get) (`self.GetActorUpVector`)) (`self.K2_GetActorLocation`)))
  (if (> (.z (`self.K2_GetActorLocation`)) 6090.0)
    (`self.K2_DestroyActor`)))

(fn `OnRep_BalloonVector`)

(fn `UserConstructionScript`)