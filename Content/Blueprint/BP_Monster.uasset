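; BP_Monster is a monster pawn that handles its own death when its HP drops below zero.
; Tick polls HP and, while a controller still exists, unpossesses it, disables actor and mesh collision, and plays AM_Monster from an offset.
; The controller validity check keeps the sequence from retriggering after unpossession.
; A short delay then destroys the actor; damage is not handled in these graphs.
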(event `self.ReceiveTick`
  (params (DeltaSeconds :type "Float (single-precision)"))
  (bind _returnvalue (`self.GetController`))
  (bind _output_get (set `self.HP` (`self.HP`)))
  (if (< _output_get 0)
    (`/Engine/EditorBlueprintResources/StandardMacros.IsValid` _returnvalue
      (:`Is Valid`
        (`Controller.UnPossess` _returnvalue)
        (`self.SetActorEnableCollision` false)
        (`PrimitiveComponent.SetCollisionEnabled` (`self.Mesh`) "NoCollision")
        (`AnimInstance.Montage_Play` (`SkeletalMeshComponent.GetAnimInstance` (`self.Mesh`)) "/Game/Animations/AM_Monster.AM_Monster" 1.0 "MontageLength" 5.68 true)
        (`KismetSystemLibrary.Delay` 2.0)
        (`self.K2_DestroyActor`)))))

(fn `UserConstructionScript`)