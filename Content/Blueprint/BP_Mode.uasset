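; BP_Mode runs a three-minute monster session, resetting player HP and spawning an initial batch of BP_Monster at random X/Y positions on BeginPlay.
; Tick counts live monsters and, after a random Delay, spawns another when fewer than ten remain.
; It prints elapsed game time, though labelled as time remaining.
; Past the limit it destroys monsters, prints a game-over message and quits after a short delay.
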(event `self.ReceiveBeginPlay`
  (set `self.PlayerHP` (`self.PlayerMAXHP`))
  (for _ (range 11)
    (`self.SpawnMonster` 0)))

(event `self.ReceiveTick`
  (params (DeltaSeconds :type "Float (single-precision)"))
  (bind _returnvalue (`KismetSystemLibrary.GetGameTimeInSeconds`))
  (`KismetSystemLibrary.PrintString` (`KismetTextLibrary.Conv_TextToString` (`|FormatText` "남은 시간  {1}초" _returnvalue)) true true (struct :`G` 0.66 :`B` 1.0 :`A` 1.0) 0.0)
  (if (<= _returnvalue 180)
    (bind _outactors (`GameplayStatics.GetAllActorsOfClass` "/Game/Blueprint/BP_Monster.BP_Monster_C"))
    (if (< (`KismetArrayLibrary.Array_Length` _outactors) 10)
      (`KismetSystemLibrary.Delay` (`KismetMathLibrary.RandomFloatInRange` 1.0 5.0))
      (`self.SpawnMonster` 0))
    (else
      (bind _outactors_2 (`GameplayStatics.GetAllActorsOfClass` "/Game/Blueprint/BP_Monster.BP_Monster_C"))
      (`self.K2_DestroyActor` _outactors_2)
      (`KismetSystemLibrary.PrintString` " 게임 종료!" true true (struct :`G` 0.66 :`B` 1.0 :`A` 1.0) 0.0)
      (`KismetSystemLibrary.Delay` 5.0)
      (`KismetSystemLibrary.QuitGame` null "Quit"))))

(fn `SpawnMonster`
  (params (NewParam :type Integer))
  (if (< NewParam 10)
    (`|SpawnActorFromClass` "/Game/Blueprint/BP_Monster.BP_Monster_C" (`KismetMathLibrary.MakeTransform` (`KismetMathLibrary.MakeVector` (`KismetMathLibrary.Conv_IntToDouble` (`KismetMathLibrary.RandomIntegerInRange` -3000 3000)) (`KismetMathLibrary.Conv_IntToDouble` (`KismetMathLibrary.RandomIntegerInRange` -3000 3000)))) "Undefined" "MultiplyWithRoot" null null)
    (return)))

(fn `UserConstructionScript`)