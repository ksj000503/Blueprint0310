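; Player character Blueprint that pops BP_Balloon actors by shooting them or touching them with its capsule.
; Fire plays the AM_Fire montage and line-traces from the screen center to find the aim point.
; A second trace runs from the mesh's FireSocket to that point and destroys any balloon it hits, with debug drawing on both traces.
; Alternative trace nodes are left unconnected, and OnRep_ShoutPoint is empty.
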(event `self.CapsuleComponent.OnComponentBeginOverlap`
  (params (OverlappedComponent :type "PrimitiveComponent Object Reference") (OtherActor :type "Actor Object Reference") (OtherComp :type "PrimitiveComponent Object Reference") (OtherBodyIndex :type Integer) (bFromSweep :type Boolean) (SweepResult :type "HitResult Structure (by ref)"))
  (bind _asbp_balloon (cast `/Game/Blueprint/BP_Balloon` OtherActor))
  (`self.K2_DestroyActor` _asbp_balloon))

(fn `Fire`
  (bind (_returnvalue_x _returnvalue_y) (`KismetMathLibrary.BreakVector2D` (`WidgetLayoutLibrary.GetViewportSize`)))
  (bind _returnvalue_location (`KismetMathLibrary.BreakTransform` (`SceneComponent.GetSocketTransform` (`self.Mesh`) "FireSocket" "RTS_World")))
  (bind (_worldposition _worlddirection) (`GameplayStatics.DeprojectScreenToWorld` (`GameplayStatics.GetPlayerController` 0) (`KismetMathLibrary.MakeVector2D` (/ _returnvalue_x 2.0) (/ _returnvalue_y 2.0))))
  (`self.PlayAnimMontage` "/Game/Animations/AM_Fire.AM_Fire")
  (bind _outhit (`KismetSystemLibrary.LineTraceSingle` :`Start` _worldposition :`End` (+ _worldposition (* _worlddirection 500000.0)) :`TraceChannel` "TraceTypeQuery1" :`DrawDebugType` "ForDuration" :`TraceColor` (struct :`R` 1.0 :`G` 0.858706 :`B` 0.806939 :`A` 1.0) :`TraceHitColor` (struct :`R` 0.677083 :`G` 0.002428 :`B` 0.017431 :`A` 1.0) :`DrawTime` 0.0))
  (bind _outhit_2 (`KismetSystemLibrary.LineTraceSingle` :`Start` _returnvalue_location :`End` (`.Location` (`GameplayStatics.BreakHitResult` _outhit)) :`TraceChannel` "TraceTypeQuery1" :`DrawDebugType` "ForDuration" :`TraceColor` (struct :`R` 1.0 :`G` 0.858706 :`B` 0.806939 :`A` 1.0) :`TraceHitColor` (struct :`R` 0.677083 :`G` 0.002428 :`B` 0.017431 :`A` 1.0)))
  (bind _asbp_balloon (cast `/Game/Blueprint/BP_Balloon` (`.HitActor` (`GameplayStatics.BreakHitResult` _outhit_2))))
  (`self.K2_DestroyActor` _asbp_balloon))

(fn `OnRep_ShoutPoint`)

(fn `UserConstructionScript`)