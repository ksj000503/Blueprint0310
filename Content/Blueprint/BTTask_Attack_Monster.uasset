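; Behavior tree task that makes a BP_Monster perform a randomly chosen attack against the player.
; It plays one of three sections of AM_Monster by starting the montage at different time offsets.
; All branches then immediately subtract one PlayerHP from the BP_Player found by class lookup, with no hit or range check, print the remaining HP, and finish successfully after a short delay.
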(event `self.ReceiveExecuteAI`
  (params (OwnerController :type "AIController Object Reference") (ControlledPawn :type "Pawn Object Reference"))
  (bind _asbp_monster (cast `/Game/Blueprint/BP_Monster` ControlledPawn))
  (switch `int` (`KismetMathLibrary.RandomIntegerInRange` 0 2)
    (:`0`
      (bind _returnvalue (`SkeletalMeshComponent.GetAnimInstance` (`Character.Mesh` _asbp_monster)))
      (`AnimInstance.Montage_Play` _returnvalue "/Game/Animations/AM_Monster.AM_Monster" 1.0 "MontageLength" 0.0 false))
    (:`1`
      (`AnimInstance.Montage_Play` _returnvalue "/Game/Animations/AM_Monster.AM_Monster" 1.0 "MontageLength" 1.84 false))
    (:`2`
      (`AnimInstance.Montage_Play` _returnvalue "/Game/Animations/AM_Monster.AM_Monster" 1.0 "MontageLength" 3.58 false)))
  (bind _returnvalue_2 (`GameplayStatics.GetActorOfClass` "/Game/Blueprint/BP_Player.BP_Player_C"))
  (set `/Game/Blueprint/BP_Player.PlayerHP` (- (`/Game/Blueprint/BP_Player.PlayerHP` _returnvalue_2) 1) _returnvalue_2)
  (`KismetSystemLibrary.PrintString` (`KismetTextLibrary.Conv_TextToString` (`|FormatText` "플레이어 체력 {0}" (`/Game/Blueprint/BP_Player.PlayerHP` _returnvalue_2))))
  (`KismetSystemLibrary.Delay` 3.0)
  (`self.FinishExecute` true))